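; BP_Storm_Street is a storm effect actor that drives Niagara systems for smoke, particles, leaves and small, big and box dump debris.
; Every Tick it looks up the BP_Wind actor and copies its wind direction, turbulence and VortexFx into user parameters on all six systems.
; It also resets their spawn rate parameter to a constant each frame, and the construction script is empty.
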(event EventTick
  (params (DeltaSeconds :type Float%20%28single-precision%29))
  (bind _niagara_storm_smoke (Variables|Default|GetNiagara_Storm_Smoke))
  (bind _returnvalue (Actor|GetActorOfClass "/Game/MsvFx_Niagara_Storm_Fx_Pack/Blueprints/BP_Wind.BP_Wind_C"))
  (Class|NiagaraComponent|SetNiagaraVariableVec3 _niagara_storm_smoke "User.WindDirection" (Variables|/Game/MsvFx_Niagara_Storm_Fx_Pack/Blueprints/BP_Wind.BP_Wind_C|GetWindDirection _returnvalue))
  (Niagara|SetNiagaraVariable(Float) _niagara_storm_smoke "User.WindTurbulance" (Variables|/Game/MsvFx_Niagara_Storm_Fx_Pack/Blueprints/BP_Wind.BP_Wind_C|GetWindTurbulance _returnvalue))
  (Niagara|SetNiagaraVariable(Float) _niagara_storm_smoke "User.Spawn_Rate" 1.0)
  (Niagara|SetNiagaraVariable(Float) (Variables|Default|GetNiagara_Storm_Particles) "User.Vortex" (Variables|/Game/MsvFx_Niagara_Storm_Fx_Pack/Blueprints/BP_Wind.BP_Wind_C|GetVortexFx _returnvalue)))

(fn ConstructionScript)